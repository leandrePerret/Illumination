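; Puzzle manager that plays a randomized sequence of lights when its SequencePlayer sends an activation.
; On BeginPlay it raises an error if LightArray is empty, otherwise builds the sequence, with settings defined only for easy mode.
; Random light indices are stored in a Set, so repeats collapse and the sequence can be shorter than requested.
; Playback passes each light an increasing delay, lighting them one after another without timers in the manager.
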(event `self.ReceiveBeginPlay`
  (bind _lightarray (`self.LightArray`))
  (bind _sequenceplayer (`self.SequencePlayer`))
  (if (`KismetArrayLibrary.Array_IsEmpty` _lightarray)
    (`KismetSystemLibrary.RaiseScriptError` (`KismetStringLibrary.Concat_StrStr` (`KismetSystemLibrary.GetDisplayName` self) " LigthArray is empty"))
    (else
      (set `self.Length` (`KismetArrayLibrary.Array_Length` _lightarray))
      (`self.InitSequence` (`self.isEasy`))
      (`/Engine/EditorBlueprintResources/StandardMacros.IsValid` _sequenceplayer
        (:`Is Valid`
          (add `/Game/Blueprint/BP_Lever_Emitter.SendActivation` _sequenceplayer (delegate `PlaySequence`)))))))

(event `InitSequence`
  (params (isEasy :type Boolean))
  (if isEasy
    (`self.InitializeSequence` 1.4 4)))

(event `PlaySequence`
  (`self.NewFunction`))

(fn `InitializeSequence`
  (params (TimeToSwitch :type "Float (double-precision)") (NumberOfIteraction :type Integer))
  (set `self.TimeToSwitch` TimeToSwitch)
  (if (not (`BlueprintSetLibrary.Set_IsEmpty` (`self.IndexArray`)))
    (`BlueprintSetLibrary.Set_Clear` (`self.IndexArray`)))
  (for _ (range NumberOfIteraction)
    (`BlueprintSetLibrary.Set_Add` (`self.IndexArray`) (`.OutIndex` (`KismetArrayLibrary.Array_Random` (`self.LightArray`))))))

(fn `NewFunction`
  (locals (CurrentIndex :type Integer))
  (set `local.CurrentIndex` 0)
  (bind _valuepin (`|SetForEach` (`self.IndexArray`))
    (:`then`
      (message `/Game/Blueprint/Puzzle/BPI_Light_Lever.TurnLightFor` (`|GetArrayItem` (`self.LightArray`) _valuepin) (* (`local.CurrentIndex`) (`self.TimeToSwitch`)) (`self.TimeToSwitch`))
      (set `local.CurrentIndex` (+ (`local.CurrentIndex`) 1)))))

(fn `UserConstructionScript`)