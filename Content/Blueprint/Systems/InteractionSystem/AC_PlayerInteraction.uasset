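; Player interaction component that finds BPI_Interactable actors ahead of the owning character and lets the player press or hold to use them.
; Each Tick runs a forward capsule trace, refreshing a screen-space prompt widget only when hit state changes.
; IA_Interact triggers Press instantly; Hold binds to a dispatcher fed by Ongoing input, filling progress until the interactable's duration passes.
; Deprecated sphere-overlap detection and closest-actor selection remain unused.
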(event `self.ReceiveBeginPlay`
  (bind _ascharacter (cast `Character` (`self.GetOwner`)))
  (`/Engine/EditorBlueprintResources/StandardMacros.IsValid` _ascharacter
    (:`Is Valid`
      (set `self.CharacterRef` _ascharacter)
      (bind _returnvalue (`|AddComponentByClass` :`self` (`self.GetOwner`) :`Class` "/Script/UMG.WidgetComponent" :`bManualAttachment` true))
      (`WidgetComponent.SetWidgetSpace` _returnvalue "Screen")
      (`WidgetComponent.SetDrawSize` _returnvalue (100.0 100.0))
      (set `self.InteractionWidgetComponent` _returnvalue))))

(event `self.ReceiveTick`
  (params (DeltaSeconds :type "Float (single-precision)"))
  ;[0 1 0.2643 0.5] New capsule trace for interactables
  (`self.UpdateInteractable` (`self.Draw Debug`)))

(event `HandleRangeBeginOverlap`
  (params (OverlappedComponent :type "PrimitiveComponent Object Reference") (OtherActor :type "Actor Object Reference") (OtherComp :type "PrimitiveComponent Object Reference") (OtherBodyIndex :type Integer) (bFromSweep :type Boolean) (SweepResult :type "HitResult Structure (by ref)"))
  ;[1 0 0 0.5] DEPRECATED CODE | Add to "InteractablesInRange" if an interactable actor is in range
  (if (`KismetSystemLibrary.DoesImplementInterface` OtherActor "/Game/Blueprint/Systems/InteractionSystem/BPI_Interactable.BPI_Interactable_C")
    (`KismetArrayLibrary.Array_AddUnique` (`self.InteractablesInRange`) OtherActor)
    (`self.RenderInteractionWidget`)))

(event `EnhancedInput|/Game/Input/Actions/IA_Interact`
  (params (ActionValue :type Boolean) (ElapsedSeconds :type "Float (double-precision)") (TriggeredSeconds :type "Float (double-precision)") (InputAction :type "InputAction Object Reference" :default "/Game/Input/Actions/IA_Interact.IA_Interact"))
  ; Interaction input Handler
  (:`Started`
    (`self.InteractBegin`) ; Press event call
  )
  (:`Ongoing`
    (`self.OnGoingInteractStart` ElapsedSeconds) ; Hold event dipatcher to avoid conflict
  )
  (:`Canceled`
    (`self.CancelInteraction` :!label _label))
  (:`Completed`
    (goto _label)))

(event `HandleRangeEndOverlap`
  (params (OverlappedComponent :type "PrimitiveComponent Object Reference") (OtherActor :type "Actor Object Reference") (OtherComp :type "PrimitiveComponent Object Reference") (OtherBodyIndex :type Integer))
  (bind _interactablesinrange (`self.InteractablesInRange`))
  ;[1 0 0 0.5] DEPRECATED CODE | Remove the interactable actor when no more in range
  (if (`KismetArrayLibrary.Array_Contains` _interactablesinrange OtherActor)
    (`KismetArrayLibrary.Array_RemoveItem` _interactablesinrange OtherActor)
    (`self.RenderInteractionWidget`)))

(event `InteractBegin`
  (bind _interactableactor (`self.InteractableActor`))
  (`/Engine/EditorBlueprintResources/StandardMacros.IsValid` _interactableactor
    (:`Is Valid`
      (bind _isactivated (message `/Game/Blueprint/Systems/InteractionSystem/BPI_Interactable.GetIsActivated` _interactableactor))
      (if _isactivated
        (bind _type (message `/Game/Blueprint/Systems/InteractionSystem/BPI_Interactable.GetInteractionType` _interactableactor))
        (switch `/Game/Blueprint/Systems/InteractionSystem/E_InteractionType` _type ; Check the type selected on object
          (:`NewEnumerator0`
            (`self.InteractWithActive`) ; Interact instantly if the Type is "Press"
          )
          (:`NewEnumerator1`
            ; When enum type is "Hold", bind an event and check if the elapsed time since pressed is greater than the wanted value
            (add `self.OnGoingInteractStart` (delegate `OnInteractionOnGoing`))))))))

(event `OnInteractionOnGoing` :!signature `self.OnGoingInteractStart`
  (params (ElapsedSeconds :type "Float (double-precision)"))
  ; When enum type is "Hold", bind an event and check if the elapsed time since pressed is greater than the wanted value
  (bind _duration (message `/Game/Blueprint/Systems/InteractionSystem/BPI_Interactable.GetHoldDuration` (`self.InteractableActor`)))
  (bind _interactionwidget (`self.InteractionWidget`)
    (:`then`
      (`/Game/UI/WB_InteractWidget.setProgressPercent` _interactionwidget (/ ElapsedSeconds _duration)))
    (:`else`
      _))
  (if (> ElapsedSeconds _duration)
    (`self.InteractWithActive`)
    (remove `self.OnGoingInteractStart` (delegate `OnInteractionOnGoing`))))

(event `InteractWithActive`
  ; Final interaction logic (called only when pressed or hold completed
  (message `/Game/Blueprint/Systems/InteractionSystem/BPI_Interactable.Interact` (`self.InteractableActor`) (`self.CharacterRef`)))

(fn `CancelInteraction`
  (bind _interactionwidget (`self.InteractionWidget`))
  (clear `self.OnGoingInteractStart`) ; Unbind all the events when the hold is completed or canceled
  (`/Engine/EditorBlueprintResources/StandardMacros.IsValid` _interactionwidget
    (:`Is Valid`
      (`/Game/UI/WB_InteractWidget.setProgressPercent` _interactionwidget 0.0))))

(fn `CreateSphereRange`
  (params (CharacterRef :type "Character Object Reference"))
  (bind _returnvalue (`|AddComponentByClass` :`self` CharacterRef :`Class` "/Script/Engine.SphereComponent"))
  (bind _output_get (set `self.RangeSphere` _returnvalue))
  (`SphereComponent.SetSphereRadius` _output_get (`self.RangeSphereRadius`) false)
  (`SceneComponent.SetHiddenInGame` _output_get (`self.NewHidden`) false))

(fn `DitanceBeetwenActors`
  (params (First :type "Actor Object Reference") (Second :type "Actor Object Reference"))
  (returns (Distance :type "Float (double-precision)"))
  (return (`KismetMathLibrary.Vector_Distance` (`Actor.K2_GetActorLocation` First) (`Actor.K2_GetActorLocation` Second))))

(fn `GetActiveInteractable`
  (returns (ActiveInteractable :type "Actor Object Reference"))
  (locals (ClosestActor :type "Actor Object Reference") (CurrentActor :type "Actor Object Reference"))
  (for (_array_element _array_index) (`self.InteractablesInRange`)
    (set `local.CurrentActor` _array_element)
    (if (== _array_index 0)
      ; If it is the first actor in array set it to closest
      (set `local.ClosestActor` (`local.CurrentActor`))
      (else
        ; Else find the closest to Character
        (set `local.ClosestActor` (`self.GetClosestActor` (`local.CurrentActor`) (`local.ClosestActor`))))))
  (return (`local.ClosestActor`)) ; End of the loop
)

(fn `GetClosestActor`
  (params (Current :type "Actor Object Reference") (Other :type "Actor Object Reference"))
  (returns (Closest :type "Actor Object Reference"))
  (bind _characterref (`self.CharacterRef`))
  (if (< (`self.DitanceBeetwenActors` Current _characterref) (`self.DitanceBeetwenActors` Other _characterref))
    (return Current) ; Return Current
    (else
      (return Other) ; Return Other
    )))

(fn `RenderInteractionWidget`
  (locals (WidgetLocation :type "Vector Structure"))
  (bind _interactableactor (`self.InteractableActor`))
  (`/Engine/EditorBlueprintResources/StandardMacros.IsValid` _interactableactor
    (:`Is Valid`
      (bind _isactivated (message `/Game/Blueprint/Systems/InteractionSystem/BPI_Interactable.GetIsActivated` _interactableactor))
      (if _isactivated
        (bind _type (message `/Game/Blueprint/Systems/InteractionSystem/BPI_Interactable.GetInteractionType` _interactableactor))
        (bind _returnvalue (`|CreateWidget` "/Game/UI/WB_InteractWidget.WB_InteractWidget_C" null _type))
        (bind _output_get (set `self.InteractionWidget` _returnvalue))
        (`WidgetComponent.SetWidget` (`self.InteractionWidgetComponent`) _output_get)
        (`|ExecutionSequence`
          (:`then_0`
            ; Verify if an offset actor is set in the interactable
            (bind _offsetcomp (message `/Game/Blueprint/Systems/InteractionSystem/BPI_Interactable.GetWidgetOffsetComp` (`self.InteractableActor`)))
            (if (`KismetSystemLibrary.IsValid` _offsetcomp)
              (set `local.WidgetLocation` (`SceneComponent.K2_GetComponentLocation` _offsetcomp))
              (else
                (set `local.WidgetLocation` (`Actor.K2_GetActorLocation` (`self.InteractableActor`))))))
          (:`then_1`
            (`SceneComponent.K2_SetWorldLocation` (`self.InteractionWidgetComponent`) (`local.WidgetLocation`) false false)))
        (else
          (`WidgetComponent.SetWidget` (`self.InteractionWidgetComponent`) null :!label _label))))
    (:`Is Not Valid`
      (goto _label))))

(fn `UpdateInteractable`
  (params (DrawDebug :type "EDrawDebugTrace Enum" :default "None"))
  (locals (PrevIsHitting :type Boolean) (DrawDebugType :type "EDrawDebugTrace Enum" :default "ForOneFrame"))
  (bind _returnvalue (`Actor.K2_GetActorLocation` (`self.CharacterRef`)))
  (bind _capsulecomponent (`Character.CapsuleComponent` (`self.CharacterRef`)))
  (bind _capsulehalfheight (`CapsuleComponent.CapsuleHalfHeight` _capsulecomponent))
  (set `local.PrevIsHitting` (`self.IsHitting`))
  (bind (_outhit _returnvalue_2) (`KismetSystemLibrary.CapsuleTraceSingle` :`Start` _returnvalue :`End` (+ _returnvalue (* (`SceneComponent.GetForwardVector` _capsulecomponent) (`self.Range`))) :`Radius` _capsulehalfheight :`HalfHeight` _capsulehalfheight :`TraceChannel` "TraceTypeQuery1" :`DrawDebugType` (`local.DrawDebug`)))
  (bind (_bblockinghit _binitialoverlap _time _distance _location _impactpoint _normal _impactnormal _physmat _hitactor) (`GameplayStatics.BreakHitResult` _outhit))
  (bind _output_get (set `self.IsHitting` (and _returnvalue_2 (`KismetSystemLibrary.DoesImplementInterface` _hitactor "/Game/Blueprint/Systems/InteractionSystem/BPI_Interactable.BPI_Interactable_C"))))
  (if _output_get
    (set `self.InteractableActor` _hitactor)
    (else
      (set `self.InteractableActor` null)))
  (if (!= (`self.IsHitting`) (`local.PrevIsHitting`))
    (`self.RenderInteractionWidget`)))