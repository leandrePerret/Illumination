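; BP_Test_Interaction is a test interactable actor that exercises the interaction system.
; On Interact, it prints an orange on-screen debug message naming the interacting actor and itself.
; It answers interaction queries with a fixed half-second hold duration, an interaction type read from its Type variable, and its Scene component as the widget offset anchor.
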(event `/Game/Blueprint/Systems/InteractionSystem/BPI_Interactable.Interact`
  (params (InteractActorRef :type "Actor Object Reference"))
  (`KismetSystemLibrary.PrintString` (`KismetStringLibrary.Concat_StrStr` (`KismetSystemLibrary.GetDisplayName` InteractActorRef) " interacting with " (`KismetSystemLibrary.GetDisplayName` self)) true false (struct :`R` 1.0 :`G` 0.396303 :`A` 1.0) 3.0))

(fn `GetHoldDuration`
  (returns (duration :type "Float (double-precision)"))
  (return 0.5))

(fn `GetInteractionType`
  (returns (Type :type "/Game/Blueprint/Systems/InteractionSystem/E_InteractionType Enum"))
  (return (`self.Type`)))

(fn `GetWidgetOffsetComp`
  (returns (OffsetComp :type "SceneComponent Object Reference"))
  (return (`self.Scene`)))

(fn `UserConstructionScript`)