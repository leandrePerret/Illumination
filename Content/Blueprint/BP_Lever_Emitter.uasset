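; Interactable lever that emits an activation signal when used and animates its handle.
; Interact only acts while the lever is not activated, setting the flag and sending activation; nothing in this Blueprint clears that flag.
; A FlipFlop then plays or reverses a timeline that lerps Cube1's pitch between an offset and its starting rotation, zeroing roll and yaw.
; Interaction getters report zero hold duration and a fixed interaction type.
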(event `self.ReceiveBeginPlay`
  (set `self.BaseRotation` (`SceneComponent.RelativeRotation` (`self.Cube1`))))

(event `/Game/Blueprint/Systems/InteractionSystem/BPI_Interactable.Interact`
  (params (InteractActorRef :type "Actor Object Reference"))
  (bind _pitch (.pitch (`self.BaseRotation`)))
  (if (not (`self.bActivated`))
    (set `self.bActivated` (not (`self.bActivated`)))
    (`self.SendActivation`)
    (`/Engine/EditorBlueprintResources/StandardMacros.FlipFlop`
      (:`A`
        (bind (_direction _levertrack) (`Timeline|Timeline` :!label _label)
          (:`Update`
            (`SceneComponent.K2_SetRelativeRotation` (`self.Cube1`) (`KismetMathLibrary.MakeRotator` 0.0 (`KismetMathLibrary.Lerp` (+ _pitch (.pitch (`self.ActivatedOffset`))) _pitch _levertrack)) false false))))
      (:`B`
        (goto _label :!via `Reverse`)))))

(fn `GetHoldDuration`
  (returns (duration :type "Float (double-precision)"))
  (return 0.0))

(fn `GetInteractionType`
  (returns (Type :type "/Game/Blueprint/Systems/InteractionSystem/E_InteractionType Enum"))
  (return "NewEnumerator0"))

(fn `GetWidgetOffsetComp`
  (returns (OffsetComp :type "SceneComponent Object Reference"))
  (return null))

(fn `UserConstructionScript`)