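; Level manager for a sequential canvas puzzle room, played in King, Queen, Valet, Princess order.
; It registers itself with each canvas, and one-shot player triggers toggle bars, light torches and activate the first canvas.
; Per-canvas verification events compare the Objects and Cards devices against hard-coded enum pairs.
; A match advances to the next canvas by toggling torches and canvas states; the last toggles the room bars and ends the level.
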(event `self.ReceiveBeginPlay`
  (set `/Game/Leandre/BP_Canvas.LevelManager` self (`self.Canvas_King`))
  (set `/Game/Leandre/BP_Canvas.LevelManager` self (`self.Canvas_Valet`))
  (set `/Game/Leandre/BP_Canvas.LevelManager` self (`self.Canvas_Queen`))
  (set `/Game/Leandre/BP_Canvas.LevelManager` self (`self.Canvas_Princess`)))

(event `self.Trigger_StartLevel.OnActorBeginOverlap`
  (params (OverlappedActor :type "Actor Object Reference") (OtherActor :type "Actor Object Reference"))
  (cast `/Game/ThirdPerson/Blueprints/BP_ThirdPersonCharacter` OtherActor)
  (`/Game/Leandre/BP_IronBars.ToggleBars` (`self.EntranceBars`))
  (`self.K2_DestroyActor` (`self.Trigger_StartLevel`)))

(event `self.Trigger_Room.OnActorBeginOverlap`
  (params (OverlappedActor :type "Actor Object Reference") (OtherActor :type "Actor Object Reference"))
  (cast `/Game/ThirdPerson/Blueprints/BP_ThirdPersonCharacter` OtherActor)
  (`/Game/Leandre/BP_IronBars.ToggleBars` (`self.CardsBars`))
  (`/Game/Leandre/BP_IronBars.ToggleBars` (`self.ObjectsBars`))
  (`/Game/Leandre/BP_IronBars.ToggleBars` (`self.RoomBars`))
  (`self.K2_DestroyActor` (`self.Trigger_Room`))
  (`/Game/Leandre/BP_Torch_Blue.On/Off Light` (`self.Torch_Room`))
  (`/Game/Leandre/BP_Torch_Red.On/Off Light` (`self.Torch_Red_King`))
  (`/Game/Leandre/BP_Canvas.ToggleState` (`self.Canvas_King`))
  (`/Game/Leandre/BP_Torch_Blue.On/Off Light` (`self.Torch_Entry`)))

(event `KingToQueen`
  (`/Game/Leandre/BP_Torch_Red.On/Off Light` (`self.Torch_Red_King`))
  (`/Game/Leandre/BP_Torch_Red.On/Off Light` (`self.Torch_Red_Queen`))
  (`/Game/Leandre/BP_Torch_Blue.On/Off Light` (`self.Torch_Blue_King`))
  (`/Game/Leandre/BP_Canvas.ToggleState` (`self.Canvas_King`))
  (`/Game/Leandre/BP_Canvas.ToggleState` (`self.Canvas_Queen`)))

(event `QueenToValet`
  (`/Game/Leandre/BP_Torch_Red.On/Off Light` (`self.Torch_Red_Queen`))
  (`/Game/Leandre/BP_Torch_Red.On/Off Light` (`self.Torch_Red_Valet`))
  (`/Game/Leandre/BP_Torch_Blue.On/Off Light` (`self.Torch_Blue_Queen`))
  (`/Game/Leandre/BP_Canvas.ToggleState` (`self.Canvas_Queen`))
  (`/Game/Leandre/BP_Canvas.ToggleState` (`self.Canvas_Valet`)))

(event `ValetToPrincess`
  (`/Game/Leandre/BP_Torch_Red.On/Off Light` (`self.Torch_Red_Valet`))
  (`/Game/Leandre/BP_Torch_Red.On/Off Light` (`self.Torch_Red_Princess`))
  (`/Game/Leandre/BP_Torch_Blue.On/Off Light` (`self.Torch_Blue_Valet`))
  (`/Game/Leandre/BP_Canvas.ToggleState` (`self.Canvas_Valet`))
  (`/Game/Leandre/BP_Canvas.ToggleState` (`self.Canvas_Princess`)))

(event `EndOfLevel`
  (`/Game/Leandre/BP_Torch_Red.On/Off Light` (`self.Torch_Red_Princess`))
  (`/Game/Leandre/BP_Torch_Blue.On/Off Light` (`self.Torch_Blue_Princess`))
  (`/Game/Leandre/BP_Torch_Blue.On/Off Light` (`self.Torch_Room`))
  (`/Game/Leandre/BP_Canvas.ToggleState` (`self.Canvas_Princess`))
  (`/Game/Leandre/BP_IronBars.ToggleBars` (`self.RoomBars`)))

(event `VerificationKing`
  (if (and (`|EnumEquality` (`/Game/Leandre/BP_Objects.CurrentValue` (`self.Dispositif_Objects`)) "NewEnumerator1") (`|EnumEquality` "NewEnumerator1" (`/Game/Leandre/BP_Cards.CurrentValue` (`self.Dispositif_Cards`))))
    (`self.KingToQueen`)))

(event `Verification Queen`
  (if (and (`|EnumEquality` (`/Game/Leandre/BP_Objects.CurrentValue` (`self.Dispositif_Objects`)) "NewEnumerator3") (`|EnumEquality` "NewEnumerator2" (`/Game/Leandre/BP_Cards.CurrentValue` (`self.Dispositif_Cards`))))
    (`self.QueenToValet`)))

(event `VerificationPrincess`
  (if (and (`|EnumEquality` (`/Game/Leandre/BP_Objects.CurrentValue` (`self.Dispositif_Objects`)) "NewEnumerator0") (`|EnumEquality` "NewEnumerator3" (`/Game/Leandre/BP_Cards.CurrentValue` (`self.Dispositif_Cards`))))
    (`self.EndOfLevel`)))

(event `VerificationValet`
  (if (and (`|EnumEquality` (`/Game/Leandre/BP_Objects.CurrentValue` (`self.Dispositif_Objects`)) "NewEnumerator2") (`|EnumEquality` "NewEnumerator0" (`/Game/Leandre/BP_Cards.CurrentValue` (`self.Dispositif_Cards`))))
    (`self.ValetToPrincess`)))

(fn `UserConstructionScript`)