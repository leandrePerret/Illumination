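; BP_Torch_Red is a torch actor with a Niagara effect and a point light that can be toggled on and off.
; Its On/OffLight event uses a FlipFlop to alternately deactivate and hide, or activate and show, the effect and light together.
; On BeginPlay it fires that toggle once if IsOn is false, so the torch starts unlit.
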(event `self.ReceiveBeginPlay`
  (if (not (`self.bIsOn`))
    (`self.On/Off Light`)))

(event `On/Off Light`
  (`/Engine/EditorBlueprintResources/StandardMacros.FlipFlop`
    (:`A`
      (`ActorComponent.Deactivate` (`self.Niagara`))
      (`SceneComponent.SetVisibility` (`self.PointLight`) false false))
    (:`B`
      (`ActorComponent.Activate` (`self.Niagara`) false)
      (`SceneComponent.SetVisibility` (`self.PointLight`) true false))))

(fn `UserConstructionScript`)