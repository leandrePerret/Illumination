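; BP_Canvas is an interactable painting that reports to the LevelManager when the player interacts with it.
; Interact switches on PaintingType (Valet, King, Queen or Princess) and calls that character's verification function on the LevelManager.
; ToggleState flips IsInteractable, which GetIsActivated returns.
; The other getters supply a fixed hold duration, an interaction type and the OffsetRoot component for widget placement.
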(event `ToggleState`
  (set `self.bIsInteractable` (not (`self.bIsInteractable`))))

(event `/Game/Blueprint/Systems/InteractionSystem/BPI_Interactable.Interact`
  (params (InteractActorRef :type "Actor Object Reference"))
  (bind _levelmanager (`self.LevelManager`))
  (switch `/Game/Enumeration/Enum_Cards` (`self.PaintingType`)
    (:`NewEnumerator0`
      (`/Game/Leandre/BP_LevelManager_Canvas.VerificationValet` _levelmanager))
    (:`NewEnumerator1`
      (`/Game/Leandre/BP_LevelManager_Canvas.VerificationKing` _levelmanager))
    (:`NewEnumerator2`
      (`/Game/Leandre/BP_LevelManager_Canvas.Verification Queen` _levelmanager))
    (:`NewEnumerator3`
      (`/Game/Leandre/BP_LevelManager_Canvas.VerificationPrincess` _levelmanager))))

(fn `GetHoldDuration`
  (returns (duration :type "Float (double-precision)"))
  (return 0.5))

(fn `GetInteractionType`
  (returns (Type :type "/Game/Blueprint/Systems/InteractionSystem/E_InteractionType Enum"))
  (return "NewEnumerator1"))

(fn `GetIsActivated`
  (returns (IsActivated :type Boolean))
  (return (`self.bIsInteractable`)))

(fn `GetWidgetOffsetComp`
  (returns (OffsetComp :type "SceneComponent Object Reference"))
  (return (`self.OffsetRoot`)))

(fn `UserConstructionScript`)